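; Sunlight Blueprint that shows its light while the player is in exterior volumes.
; Each ExteriorVolume's begin and end overlaps adjust a counter for PlayerPawn, and UpdateVisibility shows the light while it is above zero.
; BeginPlay hides the light, binds those events, then shows it for any existing PlayerPawn without touching the counter, as the initial overlap check is disconnected.
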(event `self.ReceiveBeginPlay`
  (`SceneComponent.SetVisibility` (`self.LightComponent`) false false)
  (for _array_element (`self.ExteriorVolume`)
    (`|ExecutionSequence`
      (:`then_0`
        (add `self.OnActorBeginOverlap` _array_element (delegate `CustomEvent_0`)))
      (:`then_1`
        (add `self.OnActorEndOverlap` _array_element (delegate `CustomEvent_1`)))
      (:`then_2`
        (bind _outactors (`GameplayStatics.GetAllActorsOfClass` "/Game/Cosmovania/blueprints/Entity/Pawn/PlayerPawn.PlayerPawn_C"))
        (for _array_element_2 _outactors
          (`SceneComponent.SetVisibility` (`self.LightComponent`) true false))))))

(event `CustomEvent_0` :!signature `self.OnActorBeginOverlap`
  (params (OverlappedActor :type "Actor Object Reference") (OtherActor :type "Actor Object Reference"))
  (cast `/Game/Cosmovania/blueprints/Entity/Pawn/PlayerPawn` OtherActor)
  (`/Engine/EditorBlueprintResources/StandardMacros.IncrementInt` (`self.TriggeredExteriorCount`)
    (:`  `
      (`self.UpdateVisibility`))))

(event `CustomEvent_1` :!signature `self.OnActorEndOverlap`
  (params (OverlappedActor :type "Actor Object Reference") (OtherActor :type "Actor Object Reference"))
  (cast `/Game/Cosmovania/blueprints/Entity/Pawn/PlayerPawn` OtherActor)
  (`/Engine/EditorBlueprintResources/StandardMacros.DecrementInt` (`self.TriggeredExteriorCount`)
    (:`  `
      (`self.UpdateVisibility`))))

(fn `UpdateVisibility`
  (bind _lightcomponent (`self.LightComponent`))
  (if (> (`self.TriggeredExteriorCount`) 0)
    (`SceneComponent.SetVisibility` _lightcomponent true false)
    (else
      (`SceneComponent.SetVisibility` _lightcomponent false false))))

(fn `UserConstructionScript`)