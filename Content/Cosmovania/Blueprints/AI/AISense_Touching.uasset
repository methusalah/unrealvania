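; Custom AI perception sense for touch, apparently an unfinished prototype that prints debug output.
; It stores the last registered AI controller and perception component, then binds a hit delegate on the controlled pawn during updates.
; Updates ignore incoming events, print perceived actors, register any valid Hitter as a stimuli source and request a listener update.
; No touch stimulus is built, and the controller-level hit binding is disconnected.
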(event `self.OnListenerRegistered`
  (params (ActorListener :type "Actor Object Reference") (PerceptionComponent :type "AIPerceptionComponent Object Reference"))
  (bind _asaicontroller (cast `AIController` ActorListener))
  (bind _output_get (set `self.listener` _asaicontroller))
  (set `self.perception comp` PerceptionComponent))

(event `CustomEvent_0`
  (params (SelfActor :type "Actor Object Reference") (OtherActor :type "Actor Object Reference") (NormalImpulse :type "Vector Structure") (Hit :type "HitResult Structure (by ref)"))
  (set `self.hitter` OtherActor))

(fn `OnUpdate`
  (params (EventsToProcess :type "Array of AISenseEvent Object Reference (by ref)"))
  (returns (ReturnValue :type "Float (double-precision)"))
  (`|ExecutionSequence`
    (:`then_0`
      (for _ EventsToProcess
        _))
    (:`then_1`
      (if (not (`KismetSystemLibrary.IsValid` (`self.controlled`)))
        (bind _output_get (set `self.controlled` (`Controller.K2_GetPawn` (`self.listener`))))
        (add `Actor.OnActorHit` _output_get (`|CreateDelegate` :!event `CustomEvent_0`))
        (else
          (for _array_element (`AIPerceptionComponent.GetCurrentlyPerceivedActors` (`self.perception comp`) null)
            (`KismetSystemLibrary.PrintString` (`KismetStringLibrary.Concat_StrStr` "currently" (`KismetSystemLibrary.GetDisplayName` _array_element))))
          (for _array_element_2 (`AIPerceptionComponent.GetKnownPerceivedActors` (`self.perception comp`) null)
            (`KismetSystemLibrary.PrintString` (`KismetStringLibrary.Concat_StrStr` "known" (`KismetSystemLibrary.GetDisplayName` _array_element_2))))
          (for _array_element_3 (`AIPerceptionComponent.GetPerceivedActors` (`self.perception comp`) null)
            (`KismetSystemLibrary.PrintString` (`KismetStringLibrary.Concat_StrStr` "perceived" (`KismetSystemLibrary.GetDisplayName` _array_element_3))))
          (if (`KismetSystemLibrary.IsValid` (`self.hitter`))
            (bind _returnvalue (`AIPerceptionSystem.RegisterPerceptionStimuliSource` null (`self.hitter`)))
            (`KismetSystemLibrary.PrintString` (`KismetStringLibrary.Conv_BoolToString` _returnvalue))
            (`AIPerceptionComponent.RequestStimuliListenerUpdate` (`self.perception comp`))
            (return 1.0)))))))