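; Corridor actor that procedurally lines a spline with instanced meshes at construction time, with no active gameplay logic.
; The construction script clears each CorridorInstance component and refills it along the spline using that component's spacing range.
; A helper offsets each instance left or right of the tangent, adjusts its height and randomizes tilt and yaw.
; Rotation draws from a seeded stream, but spacing uses unseeded random calls.
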(event `self.ReceiveBeginPlay`)

(fn `UserConstructionScript`
  (locals (CurrentCorridorInstance :type "/Game/Cosmovania/blueprints/env/CorridorInstance Object Reference") (Mesh :type "StaticMeshComponent Object Reference") (Distance :type "Float (double-precision)") (RandomStream :type "RandomStream Structure") (`current index` :type Integer))
  (bind _currentcorridorinstance (`local.CurrentCorridorInstance`))
  (bind _currentcorridorinstance_2 (`local.CurrentCorridorInstance`))
  (bind _randomstream (`local.RandomStream`))
  (bind _spline (`self.Spline`))
  (bind _distance (`local.Distance`))
  (bind _currentcorridorinstance_3 (`local.CurrentCorridorInstance`))
  (bind _maxtiltangle (`/Game/Cosmovania/blueprints/env/CorridorInstance.MaxTiltAngle` (`local.CurrentCorridorInstance`)))
  (bind _spacing (`/Game/Cosmovania/blueprints/env/CorridorInstance.Spacing` _currentcorridorinstance_3))
  (bind _returnvalue (* _maxtiltangle -1.0))
  (bind _returnvalue_2 (`KismetMathLibrary.Conv_IntToDouble` (`KismetMathLibrary.RandomIntegerInRange` _spacing (+ _spacing (`/Game/Cosmovania/blueprints/env/CorridorInstance.SpacingRange` _currentcorridorinstance_3)))))
  (set `local.RandomStream` (`KismetMathLibrary.MakeRandomStream` (`self.RandomSeed`)))
  (for _array_element (`self.K2_GetComponentsByClass` "/Game/Cosmovania/blueprints/env/CorridorInstance.CorridorInstance_C")
    (bind _output_get (set `local.CurrentCorridorInstance` _array_element))
    (`InstancedStaticMeshComponent.ClearInstances` _output_get)
    ;[1 1 1] Placing along spline
    (for _index (range (+ (`.ReturnValue` (`KismetMathLibrary.FMod` (`SplineComponent.GetSplineLength` (`self.Spline`)) _returnvalue_2)) 1))
      (set `local.Distance` (* _index _returnvalue_2))
      (`InstancedStaticMeshComponent.AddInstance` (`local.CurrentCorridorInstance`) (`KismetMathLibrary.MakeTransform` (+ (* (`KismetMathLibrary.Normal` (`KismetMathLibrary.GreaterGreater_VectorRotator` (`SplineComponent.GetTangentAtDistanceAlongSpline` _spline _distance "Local") (struct :`Yaw` 90.0))) (`KismetMathLibrary.Conv_IntToDouble` (* (`KismetMathLibrary.SelectInt` 1 -1 (`/Game/Cosmovania/blueprints/env/CorridorInstance.OffsetToRight` _currentcorridorinstance)) (`/Game/Cosmovania/blueprints/env/CorridorInstance.Offset` _currentcorridorinstance)))) (/ (`KismetMathLibrary.MakeVector` (.x (`SplineComponent.GetLocationAtDistanceAlongSpline` _spline _distance "Local")) (.y (`SplineComponent.GetLocationAtDistanceAlongSpline` _spline _distance "Local")) (+ (.z (`SplineComponent.GetLocationAtDistanceAlongSpline` _spline _distance "Local")) (.z (`SceneComponent.RelativeLocation` _currentcorridorinstance_2)))) (`SceneComponent.K2_GetComponentScale` _currentcorridorinstance_2))) (`KismetMathLibrary.MakeRotator` (`KismetMathLibrary.RandomFloatInRangeFromStream` _returnvalue _maxtiltangle _randomstream) (`KismetMathLibrary.RandomFloatInRangeFromStream` _returnvalue _maxtiltangle _randomstream) (`KismetMathLibrary.RandomFloatInRangeFromStream` -180.0 180.0 _randomstream)) (1.0 1.0 1.0))))))