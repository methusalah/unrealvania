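; MyCableActor is a cable actor Blueprint for Cosmovania's environment that sizes its cable automatically at construction.
; When the Test variable is above zero, the construction script sets the cable length to the distance between the actor and the cable's attached component, scaled by Test.
; Test acts as a slack multiplier, and the event graph has no runtime logic.
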(fn `UserConstructionScript`
  (if (> (`self.test`) 0.0)
    (set `CableComponent.CableLength` (* (`KismetMathLibrary.VSize` (- (`self.K2_GetActorLocation`) (`SceneComponent.K2_GetComponentLocation` (`CableComponent.GetAttachedComponent` (`self.CableComponent`))))) (`self.test`)) (`self.CableComponent`))))