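; AI controller that drives an AIPawn, running the FrigateBT behavior tree on BeginPlay.
; It caches the controlled pawn and its SenseSystem component, then copies that component's DominantPulse every tick.
; Helper functions read the blackboard Target as a PlanarPawn and return the vector from the controlled pawn to it.
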(event `self.ReceiveBeginPlay`
  (`|ExecutionSequence`
    (:`then_0`
      ;[1 1 1] Save controlled pawn
      (`self.RunBehaviorTree` "/Game/Cosmovania/blueprints/AI/frigateBT.FrigateBT")
      (bind _asaipawn (cast `/Game/Cosmovania/blueprints/Entity/Pawn/AIPawn` (`self.K2_GetPawn`))
        (:`then`
          (bind _output_get (set `self.controlledPawn` _asaipawn))
          (bind _seekedcomp (`/Game/Cosmovania/blueprints/Component/ECSLibrary.GetComponentOnOwner` "/Game/Cosmovania/Blueprints/Component/Senses/SenseSystem.SenseSystem_C" _output_get))
          (bind _assense_system (cast `/Game/Cosmovania/Blueprints/Component/Senses/SenseSystem` _seekedcomp))
          (set `self.SenseSystem` _assense_system))
        (:`CastFailed`
          (`KismetSystemLibrary.PrintString` "fuk"))))))

(event `self.ReceiveTick`
  (params (DeltaSeconds :type "Float (single-precision)"))
  (set `self.DominantPulse` (`/Game/Cosmovania/Blueprints/Component/Senses/SenseSystem.DominantPulse` (`self.SenseSystem`))))

(fn `getRecordedTarget`
  (returns (RecordedTarget :type "/Game/Cosmovania/blueprints/Entity/Pawn/PlanarPawn Object Reference"))
  (bind _returnvalue (`BlackboardComponent.GetValueAsObject` (`AIBlueprintHelperLibrary.GetBlackboard` null) "Target"))
  (if (`KismetSystemLibrary.IsValid` _returnvalue)
    (bind _asplanar_pawn (cast `/Game/Cosmovania/blueprints/Entity/Pawn/PlanarPawn` _returnvalue)
      (:`then`
        (return _asplanar_pawn))
      (:`CastFailed`
        (`KismetSystemLibrary.PrintString` "Cast error in frigate controller")
        (return null)))
    (else
      (return null))))

(fn `getVectorToTarget`
  (returns (`Vector to Target` :type "Vector Structure"))
  (bind _recordedtarget (`self.getRecordedTarget`))
  (return (- (`self.K2_GetActorLocation` _recordedtarget) (`self.K2_GetActorLocation` (`self.K2_GetPawn`)))))

(fn `UserConstructionScript`)