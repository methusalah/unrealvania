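; Actor component that tracks whether an ability is active based on commands held by the owner's EventSystem component.
; On BeginPlay it finds and caches the owner's EventSystem component.
; Each Tick it sets Activated to whether that component's Command collection contains this ability's own Command.
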(event `self.ReceiveBeginPlay`
  (bind _seekedcomp (`/Game/Cosmovania/blueprints/Component/ECSLibrary.GetComponentOnOwner` "/Game/Cosmovania/blueprints/Component/EventSystem.EventSystem_C" (`self.GetOwner` self)))
  (bind _asevent_system (cast `/Game/Cosmovania/blueprints/Component/EventSystem` _seekedcomp))
  (set `self.EventSystem` _asevent_system))

(event `self.ReceiveTick`
  (params (DeltaSeconds :type "Float (single-precision)"))
  (set `self.Activated` (`KismetArrayLibrary.Array_Contains` (`/Game/Cosmovania/blueprints/Component/EventSystem.Command` (`self.EventSystem`)) (`self.Command`))))