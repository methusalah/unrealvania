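; ECSLibrary is a helper library with one function, GetComponentOnOwner, that finds the single component of a given class belonging to an actor.
; When the actor does not hold exactly one match, the lookup recurses up the parent actor chain, covering actors spawned through Child Actor Components.
; If the chain ends without a unique match, it prints an on-screen error naming the class and the last actor searched.
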(fn `GetComponentOnOwner`
  (params (ComponentClass :type "ActorComponent Class Reference") (Owner :type "Actor Object Reference"))
  (returns (SeekedComp :type "ActorComponent Object Reference"))
  (bind _returnvalue (`Actor.K2_GetComponentsByClass` Owner ComponentClass))
  (bind _returnvalue_2 (`Actor.GetParentActor` Owner))
  (if (!= (`KismetArrayLibrary.Array_Length` _returnvalue) 1)
    (if (`KismetSystemLibrary.IsValid` _returnvalue_2)
      (bind _seekedcomp (`self.GetComponentOnOwner` ComponentClass _returnvalue_2))
      (return _seekedcomp)
      (else
        (`KismetSystemLibrary.PrintString` null (`KismetStringLibrary.Concat_StrStr` "Impossible to find one (and only one) " (`KismetSystemLibrary.GetClassDisplayName` ComponentClass) " on actor " (`KismetSystemLibrary.GetDisplayName` Owner)) true true (struct :`R` 1.0 :`B` 0.114395 :`A` 1.0) 10.0)))
    (else
      (return (`KismetArrayLibrary.Array_Get` _returnvalue)))))