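; RetrySystem is a checkpoint respawn component that returns its owner to the last activated RetryBooth after it decays.
; A sphere collision, required as first child, detects overlapped booths, switching off the previous one and activating the new one.
; It listens to the Decay event on the owner's EventSystem, waits briefly, then calls Revive, moves the owner to the booth and zeroes its physics velocity.
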(event `CustomEvent_1`
  (params (OverlappedComponent :type "PrimitiveComponent Object Reference") (OtherActor :type "Actor Object Reference") (OtherComp :type "PrimitiveComponent Object Reference") (OtherBodyIndex :type Integer) (bFromSweep :type Boolean) (SweepResult :type "HitResult Structure (by ref)"))
  (bind _asretry_booth (cast `/Game/Cosmovania/Blueprints/env/RetryBooth` OtherActor))
  (`/Game/Cosmovania/Blueprints/env/RetryBooth.SetActivated` (`self.Booth`) false)
  (bind _output_get (set `self.Booth` _asretry_booth))
  (`/Game/Cosmovania/Blueprints/env/RetryBooth.SetActivated` _output_get true)
  (`KismetSystemLibrary.PrintString` "booth activated"))

(event `self.ReceiveBeginPlay`
  (`|ExecutionSequence`
    (:`then_0`
      (bind _assphere_collision (cast `SphereComponent` (`self.GetChildComponent` self 0))
        (:`then`
          (add `PrimitiveComponent.OnComponentBeginOverlap` _assphere_collision (delegate `CustomEvent_1`)))
        (:`CastFailed`
          (`KismetSystemLibrary.PrintString` "RetrySystem needs a sphere collision as first child"))))
    (:`then_1`
      (bind _seekedcomp (`/Game/Cosmovania/blueprints/Component/ECSLibrary.GetComponentOnOwner` "/Game/Cosmovania/blueprints/Component/EventSystem.EventSystem_C" (`self.GetOwner`)))
      (bind _asevent_system (cast `/Game/Cosmovania/blueprints/Component/EventSystem` _seekedcomp))
      (bind _output_get (set `self.EventSystem` _asevent_system))
      (add `/Game/Cosmovania/blueprints/Component/EventSystem.Decay` _output_get (delegate `CustomEvent_2`)))))

(event `CustomEvent_2`
  (`KismetSystemLibrary.K2_SetTimerDelegate` (delegate `CustomEvent_0`) 3.0))

(event `CustomEvent_0`
  (bind _returnvalue (`self.GetOwner` self))
  (`/Game/Cosmovania/blueprints/Component/EventSystem.Revive` (`self.EventSystem`))
  (`Actor.K2_SetActorLocation` _returnvalue (`Actor.K2_GetActorLocation` (`self.Booth`)) false false)
  (bind _asprimitive_component (cast `PrimitiveComponent` (`Actor.K2_GetRootComponent` _returnvalue)))
  (`PrimitiveComponent.SetAllPhysicsLinearVelocity` _asprimitive_component (0.0 0.0 0.0) false))